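; BP_1_Tunnel is a tunnel floor tile for an endless track driven by a MonsterTruck.
; Construction randomly adds either a blocker at one of three spawn points (two in three odds) or gas at a random point inside GasArea.
; When the truck overlaps EndTrigger, the tile asks VehicleGameMode to add a floor tile, then destroys itself after a short delay.
; GetAttachTransform exposes the AttachPoint world transform.
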(event `self.ReceiveBeginPlay`)

(event `self.ReceiveActorBeginOverlap`
  (params (OtherActor :type "Actor Object Reference")))

(event `self.ReceiveTick`
  (params (DeltaSeconds :type "Float (single-precision)")))

(event `self.EndTrigger.OnComponentBeginOverlap`
  (params (OtherActor :type "Actor Object Reference") (OtherComp :type "PrimitiveComponent Object Reference") (OtherBodyIndex :type Integer) (bFromSweep :type Boolean) (SweepResult :type "HitResult Structure (by ref)"))
  ;[1 1 1] Adds and destroy floor actor
  (cast `/Game/MyContent/BluePrints/VehicleBP/MonsterTruck/MonsterTruck` OtherActor)
  (bind _asvehicle_game_mode (cast `/Game/MyContent/BluePrints/VehicleBP/Blueprints/VehicleGameMode` (`GameplayStatics.GetGameMode`)))
  (`/Game/MyContent/BluePrints/VehicleBP/Blueprints/VehicleGameMode.AddFloorTile` _asvehicle_game_mode)
  (`KismetSystemLibrary.Delay` 2.0)
  (`self.K2_DestroyActor`))

(fn `GetAttachTransform`
  (returns (AttachTransform :type "Transform Structure"))
  (return (`SceneComponent.K2_GetComponentToWorld` (`self.AttachPoint`))))

(fn `SetSpawnPoints`
  (set `self.SpawnPoints` (`|MakeArray` (`SceneComponent.GetRelativeTransform` (`self.SpawnPointL`)) (`SceneComponent.GetRelativeTransform` (`self.SpawnPointR`)) (`SceneComponent.GetRelativeTransform` (`self.SpawnPoint`)))))

(fn `SpawnBlocker`
  (bind _spawnpoints (`self.SpawnPoints`))
  (`AddComponent|Child Actor Component_0` :`RelativeTransform` (`KismetArrayLibrary.Array_Get` _spawnpoints (`KismetMathLibrary.RandomIntegerInRange` 0 (`KismetArrayLibrary.Array_LastIndex` _spawnpoints)))))

(fn `SpawnGas`
  (bind _gasarea (`self.GasArea`))
  (`AddComponent|Child Actor Component_1` :`RelativeTransform` (`KismetMathLibrary.Conv_VectorToTransform` (`KismetMathLibrary.RandomPointInBoundingBox` (`SceneComponent.RelativeLocation` _gasarea) (`BoxComponent.BoxExtent` _gasarea)))))

(fn `UserConstructionScript`
  ;[1 1 1] Spawns The Collectables and Obstacles
  (`self.SetSpawnPoints`)
  (switch `int` (`KismetMathLibrary.RandomIntegerInRange` 0 5)
    (:`Default`
      (`self.SpawnBlocker` :!label _label))
    (:`0`
      (goto _label))
    (:`1`
      (goto _label))
    (:`2`
      (goto _label))
    (:`3`
      (goto _label))
    (:`4`
      (`self.SpawnGas` :!label _label_2))
    (:`5`
      (goto _label_2))))