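; Gasoline is a collectable pickup that rewards the player's monster truck with score and fuel.
; On overlap with a MonsterTruck, it adds its gas score value to the VehicleGameMode score and raises gas progress by a fixed step, clamped to a maximum.
; It then destroys itself; all state lives on the game mode, and no other events do any work.
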(event `self.ReceiveBeginPlay`)

(event `self.ReceiveActorBeginOverlap`
  (params (OtherActor :type "Actor Object Reference")))

(event `self.ReceiveTick`
  (params (DeltaSeconds :type "Float (single-precision)")))

(event `self.ReceiveActorBeginOverlap`
  (params (OtherActor :type "Actor Object Reference"))
  ;[1 1 1] OnCollision
  (cast `/Game/MyContent/BluePrints/VehicleBP/MonsterTruck/MonsterTruck` OtherActor)
  (bind _asvehicle_game_mode (cast `/Game/MyContent/BluePrints/VehicleBP/Blueprints/VehicleGameMode` (`GameplayStatics.GetGameMode`)))
  (set `/Game/MyContent/BluePrints/VehicleBP/Blueprints/VehicleGameMode.Score` (+ (`self.GasScoreValue`) (`/Game/MyContent/BluePrints/VehicleBP/Blueprints/VehicleGameMode.Score` _asvehicle_game_mode)) _asvehicle_game_mode)
  (bind _returnvalue (+ (`/Game/MyContent/BluePrints/VehicleBP/Blueprints/VehicleGameMode.GasProgress` _asvehicle_game_mode) 0.1))
  (if (>= _returnvalue (`self.maxGasProgress`))
    (set `/Game/MyContent/BluePrints/VehicleBP/Blueprints/VehicleGameMode.GasProgress` (`self.maxGasProgress`) _asvehicle_game_mode)
    (else
      (set `/Game/MyContent/BluePrints/VehicleBP/Blueprints/VehicleGameMode.GasProgress` _returnvalue _asvehicle_game_mode)))
  (`self.K2_DestroyActor`))

(fn `UserConstructionScript`)